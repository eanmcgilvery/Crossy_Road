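; One ground row in an endless Crossy Road-style game, which sets its mesh and spawns matching scenery or hazards.
; RandomizeGround makes the first rows grass with foliage, then randomly picks grass, road with vehicles, rail with trains, or water with logs or lily pads.
; The chicken hitting SpawnTrigger has GenerateGround add a row and drop the oldest.
; Other triggers recycle red cars, logs and trains by spawning replacements and destroying arrivals, with trains randomly delayed.
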(event OnComponentBeginOverlap(CarTrigger)
  (params (OverlappedComponent :type Primitive%20Component%20Object%20Reference) (OtherActor :type Actor%20Object%20Reference) (OtherComp :type Primitive%20Component%20Object%20Reference) (OtherBodyIndex :type Integer) (bFromSweep :type Boolean) (SweepResult :type Hit%20Result%20Structure%20%28by%20ref%29))
  (Utilities|Casting|CastToBP_RedCar OtherActor)
  (CallFunction|SpawnCar (Math|Vector|MakeVector (.x (Transformation|GetActorLocation)) 5e+02 1.5e+02))
  (Audio|PlaySound2D "/Game/Blueprints/carSound1.carSound1" 1.0 1.0 0.0 0 0)
  (Actor|DestroyActor OtherActor))

(event OnComponentBeginOverlap(SpawnTrigger)
  (params (OverlappedComponent :type Primitive%20Component%20Object%20Reference) (OtherActor :type Actor%20Object%20Reference) (OtherComp :type Primitive%20Component%20Object%20Reference) (OtherBodyIndex :type Integer) (bFromSweep :type Boolean) (SweepResult :type Hit%20Result%20Structure%20%28by%20ref%29))
  (Utilities|Casting|CastToChikcen OtherActor)
  (Default|SpawnGroundatSpawnPoint (Variables|Default|GetGenerateGround))
  (Components|DestroyComponent (Variables|Default|GetSpawnTrigger))
  (Default|DestroyOldestGround (Variables|Default|GetGenerateGround) self))

(event OnComponentBeginOverlap(LogTrigger)
  (params (OverlappedComponent :type Primitive%20Component%20Object%20Reference) (OtherActor :type Actor%20Object%20Reference) (OtherComp :type Primitive%20Component%20Object%20Reference) (OtherBodyIndex :type Integer) (bFromSweep :type Boolean) (SweepResult :type Hit%20Result%20Structure%20%28by%20ref%29))
  (Utilities|Casting|CastToBP_Log OtherActor)
  (CallFunction|SpawnLog (Math|Vector|MakeVector (.x (Transformation|GetActorLocation)) 5e+02 1e+02))
  (Actor|DestroyActor OtherActor))

(event OnComponentBeginOverlap(TrainTrigger)
  (params (OverlappedComponent :type Primitive%20Component%20Object%20Reference) (OtherActor :type Actor%20Object%20Reference) (OtherComp :type Primitive%20Component%20Object%20Reference) (OtherBodyIndex :type Integer) (bFromSweep :type Boolean) (SweepResult :type Hit%20Result%20Structure%20%28by%20ref%29))
  (Utilities|FlowControl|Delay (Math|Random|RandomFloatinRange 7.0 2e+01))
  (Utilities|Casting|CastToBP_Train OtherActor)
  (CallFunction|SpawnTrain (Math|Vector|MakeVector (.x (Transformation|GetActorLocation)) -1e+03 2e+02))
  (Audio|PlaySound2D "/Game/Blueprints/trainSound.trainSound" 1.0 1.0 0.0 0 0)
  (Actor|DestroyActor OtherActor))

(event EventBeginPlay)

(event Collision|EventActorBeginOverlap
  (params (OtherActor :type Actor%20Object%20Reference)))

(event EventTick
  (params (DeltaSeconds :type Float%20%28single-precision%29)))

(fn ConstructionScript)

(fn DestroyTrigger
  (Utilities|IsValid (Variables|Default|GetSpawnTrigger)
    (:Is%20Valid
      (Components|DestroyComponent (Variables|Default|GetSpawnTrigger)))))

(fn DestroyGround
  (Utilities|IsValid (Variables|Default|GetFoliage)
    (:Is%20Valid
      (Default|KillMe (Variables|Default|GetFoliage)))
    (:Is%20Not%20Valid
      _))
  (for (_ _array_index) (Variables|Default|GetLilyPad)
    (if (Utilities|Array|IsValidIndex (Variables|Default|GetLilyPad) _array_index)
      (Default|KillMe (Utilities|Array|Get(acopy) (Variables|Default|GetLilyPad) _array_index))))
  (Actor|DestroyActor))

(fn RandomizeGround
  (params (GroundCounter :type Integer))
  (bind _returnvalue (Transformation|GetActorLocation))
  (if (< GroundCounter 10)
    (bind _output_get (Variables|Default|SetgroundType (Math|Integer|%(Integer) GroundCounter 2)))
    (if (Utilities|Select :Index (Math|Random|RandomInteger 2) :Option%200 false :Option%201 true)
      (CallFunction|SpawntheFoliage (Math|Vector|MakeVector (.x (Transformation|GetActorLocation)) (Math|Random|RandomFloatinRange -2.5e+03 -7.5e+02) 0.0))
      (else
        (CallFunction|SpawntheFoliage (Math|Vector|MakeVector (.x (Transformation|GetActorLocation)) (Math|Random|RandomFloatinRange 2.5e+02 2e+03) 0.0))))
    (Components|StaticMesh|SetStaticMesh (Variables|Default|GetGroundMesh) (Utilities|Select :Index _output_get :Option%200 "/Game/Meshes/grass1.grass1" :Option%201 "/Game/Meshes/grass3.grass3"))
    (else
      (bind _output_get_2 (Variables|Default|SetRandInt (Math|Random|RandomInteger 5)))
      (if (== _output_get_2 2)
        (CallFunction|SpawnCar (Math|Vector|MakeVector (.x _returnvalue) 0.0 0.0))
        (elif (== _output_get_2 4)
          (if (== (Math|Random|RandomInteger 2) 0)
            (CallFunction|SpawntheLillies)
            (else
              (CallFunction|SpawnLog (Math|Vector|MakeVector (.x _returnvalue) 0.0 0.0))))
          (elif (== _output_get_2 3)
            (CallFunction|SpawnTrain (Math|Vector|MakeVector (.x _returnvalue) 0.0 0.0))
            (elif (< _output_get_2 2)
              (CallFunction|SpawntheFoliage (Math|Vector|MakeVector (.x (Transformation|GetActorLocation)) (Math|Random|RandomFloatinRange -2.5e+03 2e+03) 0.0))))))
      (Components|StaticMesh|SetStaticMesh (Variables|Default|GetGroundMesh) (Utilities|Select :Index _output_get_2 :Option%200 "/Game/Meshes/grass1.grass1" :Option%201 "/Game/Meshes/grass3.grass3" :Option%202 "/Game/Meshes/road.road" :Option%203 "/Game/Meshes/RR_track_1.RR_track_1" :Option%204 "/Game/Meshes/water.water")))))

(fn SpawntheFoliage
  (params (Location :type Vector))
  (bind _returnvalue (Game|SpawnActorfromClass "/Game/Blueprints/BP_Foliage.BP_Foliage_C" (Math|Transform|MakeTransform (Math|Vector|MakeVector (.x Location) (.y Location) 1.5e+02) "0,-90.000000, 0" "1,1,1") "Undefined" 0 0))
  (bind _output_get (Variables|Default|SetFoliage _returnvalue))
  (if (> (Variables|/Game/Blueprints/BP_Foliage.BP_Foliage_C|GetFoliageType _output_get) 2)
    (Transformation|AddActorWorldOffset (Variables|Default|GetFoliage) (Math|Vector|MakeVector -1e+02 0.0 0.0))))

(fn SpawntheLillies
  (for _index (range 0 (Math|Random|RandomInteger 6))
    (bind _output_get (LocalVariables|SetRandLoc (Math|Random|RandomFloatinRange -2.5e+03 2e+03)))
    (bind _returnvalue (Game|SpawnActorfromClass "/Game/Blueprints/BP_LilyPad.BP_LilyPad_C" (Math|Transform|MakeTransform (Math|Vector|MakeVector (.x (Transformation|GetActorLocation)) _output_get 1.2e+02) "0,-90.000000, 0" "1,1,1") "Undefined" 0 0))
    (Utilities|Array|Add (Variables|Default|GetLilyPad) _returnvalue)))

(fn SpawnCar
  (params (Spawn%20Location :type Vector))
  (bind _returnvalue (Math|Random|RandomIntegerinRange 0 2))
  (if (== _returnvalue 0)
    (bind _returnvalue_2 (Game|SpawnActorfromClass "/Game/Blueprints/BP_RedCar.BP_RedCar_C" (Math|Transform|MakeTransform (Math|Vector|MakeVector (.x Spawn%20Location) 2.5e+03 1.5e+02) "0.000000,-90.000000,0.000000" "3.000000,3.000000,3.000000") "Undefined" 0 0))
    (bind _output_get (Variables|Default|SettempCar _returnvalue_2))
    (Utilities|Array|Add (Variables|Default|GetCarArr) _output_get)
    (elif (== _returnvalue 1)
      (bind _returnvalue_3 (Game|SpawnActorfromClass "/Game/Blueprints/BP_YellowCar.BP_YellowCar_C" (Math|Transform|MakeTransform (Math|Vector|MakeVector (.x Spawn%20Location) 2.5e+03 1.5e+02) "0,-90.000000, 0" "3.000000,3.000000,3.000000") "Undefined" 0 0))
      (bind _output_get_2 (Variables|Default|SettempYCar _returnvalue_3))
      (Utilities|Array|Add (Variables|Default|GetYCarArr) _output_get_2)
      (elif (== _returnvalue 2)
        (bind _returnvalue_4 (Game|SpawnActorfromClass "/Game/Blueprints/BP_RedCar_2.BP_RedCar_2_C" (Math|Transform|MakeTransform (Math|Vector|MakeVector (.x Spawn%20Location) 2.5e+03 1.5e+02) "0.000000,-90.000000,0.000000" "6.000000,6.000000,6.000000") "Undefined" 0 0))
        (bind _output_get_3 (Variables|Default|SettempTruck _returnvalue_4))
        (Utilities|Array|Add (Variables|Default|GettruckArr) _output_get_3)))))

(fn SpawnTrain
  (params (Spawn%20Location :type Vector))
  (bind _returnvalue (Game|SpawnActorfromClass "/Game/Blueprints/BP_Train.BP_Train_C" (Math|Transform|MakeTransform (Math|Vector|MakeVector (.x Spawn%20Location) 2.5e+03 1.5e+02) "0.000000,-90.000000,0.000000" "1.500000,1.500000,1.500000") "Undefined" 0 0))
  (bind _output_get (Variables|Default|SettempTrain _returnvalue))
  (Utilities|Array|Add (Variables|Default|GetTrainArr) _output_get))

(fn SpawnLog
  (params (StartLocation :type Vector))
  (bind _returnvalue (Math|Random|RandomIntegerinRange 0 2))
  (if (== _returnvalue 0)
    (bind _returnvalue_2 (Game|SpawnActorfromClass "/Game/Blueprints/BP_Log.BP_Log_C" (Math|Transform|MakeTransform (Math|Vector|MakeVector (.x StartLocation) 2.5e+03 1e+02) "0.000000,-90.000000,0.000000" "5.000000,5.000000,5.000000") "Undefined" 0 0))
    (elif (== _returnvalue 1)
      (Game|SpawnActorfromClass "/Game/Blueprints/BP_Log_2.BP_Log_2_C" (Math|Transform|MakeTransform (Math|Vector|MakeVector 0.0 2.5e+03 1e+02) "0.000000,-90.000000,0.000000" "5.000000,5.000000,5.000000") "Undefined" 0 0)
      (else
        (Game|SpawnActorfromClass "/Game/Blueprints/BP_Log_3.BP_Log_3_C" (Math|Transform|MakeTransform (Math|Vector|MakeVector 0.0 2.5e+03 1e+02) "0.000000,-90.000000,0.000000" "5.000000,5.000000,5.000000") "Undefined" 0 0))))
  (bind _output_get (Variables|Default|SettempLog _returnvalue_2)))