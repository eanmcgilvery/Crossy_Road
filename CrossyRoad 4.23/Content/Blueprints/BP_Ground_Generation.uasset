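; BP_Ground_Generation is a manager that builds and recycles a chain of BP_Ground segments, starting beneath the player.
; On BeginPlay it spawns an initial run, each at the previous segment's SpawnPoint, removing triggers from the earliest ones.
; Each segment receives a back-reference and is randomized using a running counter.
; DestroyOldestGround removes the tail segment and shifts a fixed window of trailing references to take in the current one.
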(event EventBeginPlay
  (CallFunction|SpawnInitialGround))

(event Collision|EventActorBeginOverlap
  (params (OtherActor :type Actor%20Object%20Reference)))

(event EventTick
  (params (DeltaSeconds :type Float%20%28single-precision%29)))

(fn ConstructionScript)

(fn SpawnGround
  (params (SpawnLocation :type Vector))
  (bind _returnvalue (Game|SpawnActorfromClass "/Game/Blueprints/BP_Ground.BP_Ground_C" (Math|Transform|MakeTransform SpawnLocation "0, 0, 0" "1,1,1") "Undefined" 0 0))
  (bind _output_get (Variables|Default|SetNewestGround _returnvalue))
  (Variables|/Game/Blueprints/BP_Ground.BP_Ground_C|SetGenerateGround _output_get self)
  (Default|RandomizeGround (Variables|Default|GetNewestGround) (Variables|Default|GetGroundCounter))
  (Math|Integer|IncrementInt (Variables|Default|GetGroundCounter)))

(fn SpawnInitialGround
  (for _index (range 0 40)
    (Utilities|IsValid (Variables|Default|GetNewestGround)
      (:Is%20Valid
        (CallFunction|SpawnGroundatSpawnPoint)
        (if (< _index 5)
          (Default|DestroyTrigger (Variables|Default|GetNewestGround))
          (if (== _index 1)
            (Variables|Default|SetOldGround1 (Variables|Default|GetNewestGround))
            (elif (== _index 2)
              (Variables|Default|SetOldGround2 (Variables|Default|GetNewestGround))
              (elif (== _index 3)
                (Variables|Default|SetOldGround3 (Variables|Default|GetNewestGround))
                (elif (== _index 4)
                  (Variables|Default|SetOldGround4 (Variables|Default|GetNewestGround))))))
          (elif (== _index 5)
            (Variables|Default|SetOldGround5 (Variables|Default|GetNewestGround)))))
      (:Is%20Not%20Valid
        (CallFunction|SpawnGround (+ (Transformation|GetActorLocation (Game|Player|GetPlayerPawn 0)) "0.000000,0.000000,-200.000000"))
        (Default|DestroyTrigger (Variables|Default|GetNewestGround))
        (Variables|Default|SetOldestGround (Variables|Default|GetNewestGround))))))

(fn SpawnGroundatSpawnPoint
  (CallFunction|SpawnGround (Transformation|GetWorldLocation (Variables|/Game/Blueprints/BP_Ground.BP_Ground_C|GetSpawnPoint (Variables|Default|GetNewestGround)))))

(fn DestroyOldestGround
  (params (CurrentGround :type BP%20Ground%20Object%20Reference))
  (Utilities|IsValid (Variables|Default|GetOldestGround)
    (:Is%20Valid
      (Default|DestroyGround (Variables|Default|GetOldestGround)))
    (:Is%20Not%20Valid
      _))
  (Variables|Default|SetOldestGround (Variables|Default|GetOldGround1))
  (Variables|Default|SetOldGround1 (Variables|Default|GetOldGround2))
  (Variables|Default|SetOldGround2 (Variables|Default|GetOldGround3))
  (Variables|Default|SetOldGround3 (Variables|Default|GetOldGround4))
  (Variables|Default|SetOldGround4 (Variables|Default|GetOldGround5))
  (Variables|Default|SetOldGround5 CurrentGround))