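; Player-controlled chicken character that hops in four directions and also moves with forward and right axis input.
; Pressing a directional jump squashes the mesh; releasing restores it, jumps, adds movement input and snaps the mesh to face that way, with hard-coded offsets per previous rotation.
; Tick consumes the movement input and applies it as a scaled, unswept local offset.
; The movability and key-press functions are empty stubs, and the Rotation function is not called here.
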(event EventBeginPlay)

(event Collision|EventActorBeginOverlap
  (params (OtherActor :type Actor%20Object%20Reference)))

(event EventTick
  (params (DeltaSeconds :type Float%20%28single-precision%29))
  (bind _returnvalue (Class|Pawn|ConsumeMovementInputVector))
  (Transformation|AddActorLocalOffset (* _returnvalue 5.0) false false))

(event Input|ActionEvents|InputActionJumpBackward
  (params (Key :type Key%20Structure :default "None"))
  (:Pressed
    (Transformation|SetWorldTransform (Variables|Character|GetStaticMesh) (Math|Transform|MakeTransform (Transformation|GetWorldLocation (Variables|Character|GetStaticMesh)) (Transformation|GetWorldRotation (Variables|Character|GetStaticMesh)) "3.000000,2.700000,3.000000") false false))
  (:Released
    (Transformation|SetWorldTransform (Variables|Character|GetStaticMesh) (Math|Transform|MakeTransform (Transformation|GetWorldLocation (Variables|Character|GetStaticMesh)) (Transformation|GetWorldRotation (Variables|Character|GetStaticMesh)) "3.000000,3.000000,3.000000") false false)
    (Character|Jump)
    (Pawn|Input|AddMovementInput (- (Transformation|GetActorForwardVector) "500.000000, 0, 0") 1.0 false)
    (if (Math|Rotator|Equal(Rotator) (Transformation|GetWorldRotation (Variables|Character|GetStaticMesh)) "0,90.000000,90.000000" 0.0001)
      (Transformation|SetWorldLocationAndRotation (Variables|Character|GetStaticMesh) (+ (Transformation|GetWorldLocation (Variables|Character|GetStaticMesh)) "300.000000,-300.000000, 0") "0,270.000000,90.000000" false false)
      (elif (Math|Rotator|Equal(Rotator) (Transformation|GetWorldRotation (Variables|Character|GetStaticMesh)) "0,180.000000,90.000000" 0.0001)
        (Transformation|SetWorldLocationAndRotation (Variables|Character|GetStaticMesh) (+ (Transformation|GetWorldLocation (Variables|Character|GetStaticMesh)) "300.000000,0.000000, 0") "0,270.000000,90.000000" false false)
        (elif (Math|Rotator|Equal(Rotator) (Transformation|GetWorldRotation (Variables|Character|GetStaticMesh)) "0, 0,90.000000" 0.0001)
          (Transformation|SetWorldLocationAndRotation (Variables|Character|GetStaticMesh) (+ (Transformation|GetWorldLocation (Variables|Character|GetStaticMesh)) "0.000000,-300.000000, 0") "0,270.000000,90.000000" false false))))))

(event Input|ActionEvents|InputActionJump
  (params (Key :type Key%20Structure :default "None"))
  (:Released
    (Character|Jump)
    (Pawn|Input|AddMovementInput (+ (Transformation|GetActorForwardVector) "150.000000, 0, 0") 5.0 false)))

(event Input|ActionEvents|InputActionJumpForward
  (params (Key :type Key%20Structure :default "None"))
  (:Pressed
    (Transformation|SetWorldTransform (Variables|Character|GetStaticMesh) (Math|Transform|MakeTransform (Transformation|GetWorldLocation (Variables|Character|GetStaticMesh)) (Transformation|GetWorldRotation (Variables|Character|GetStaticMesh)) "3.000000,2.700000,3.000000") false false))
  (:Released
    (Transformation|SetWorldTransform (Variables|Character|GetStaticMesh) (Math|Transform|MakeTransform (Transformation|GetWorldLocation (Variables|Character|GetStaticMesh)) (Transformation|GetWorldRotation (Variables|Character|GetStaticMesh)) "3.000000,3.000000,3.000000") false false)
    (Character|Jump)
    (Pawn|Input|AddMovementInput (+ (Transformation|GetActorForwardVector) "500.000000, 0, 0") 1.0 false)
    (if (Math|Rotator|Equal(Rotator) (Transformation|GetWorldRotation (Variables|Character|GetStaticMesh)) "0,270.000000,90.000000" 0.0001)
      (Transformation|SetWorldLocationAndRotation (Variables|Character|GetStaticMesh) (+ (Transformation|GetWorldLocation (Variables|Character|GetStaticMesh)) "-300.000000,300.000000, 0") "0,90.000000,90.000000" false false)
      (elif (Math|Rotator|Equal(Rotator) (Transformation|GetWorldRotation (Variables|Character|GetStaticMesh)) "0,180.000000,90.000000" 0.0001)
        (Transformation|SetWorldLocationAndRotation (Variables|Character|GetStaticMesh) (+ (Transformation|GetWorldLocation (Variables|Character|GetStaticMesh)) "0.000000,300.000000, 0") "0,90.000000,90.000000" false false)
        (elif (Math|Rotator|Equal(Rotator) (Transformation|GetWorldRotation (Variables|Character|GetStaticMesh)) "0, 0,90.000000" 0.0001)
          (Transformation|SetWorldLocationAndRotation (Variables|Character|GetStaticMesh) (+ (Transformation|GetWorldLocation (Variables|Character|GetStaticMesh)) "-300.000000,0.000000, 0") "0,90.000000,90.000000" false false))))))

(event Input|ActionEvents|InputActionBackJump
  (params (Key :type Key%20Structure :default "None"))
  (:Released
    (Character|Jump)
    (Pawn|Input|AddMovementInput (- (Transformation|GetActorForwardVector) "150.000000, 0, 0") 1.0 false)))

(event Input|ActionEvents|InputActionJumpLeft
  (params (Key :type Key%20Structure :default "None"))
  (:Pressed
    (Transformation|SetWorldTransform (Variables|Character|GetStaticMesh) (Math|Transform|MakeTransform (Transformation|GetWorldLocation (Variables|Character|GetStaticMesh)) (Transformation|GetWorldRotation (Variables|Character|GetStaticMesh)) "3.000000,2.700000,3.000000") false false))
  (:Released
    (Transformation|SetWorldTransform (Variables|Character|GetStaticMesh) (Math|Transform|MakeTransform (Transformation|GetWorldLocation (Variables|Character|GetStaticMesh)) (Transformation|GetWorldRotation (Variables|Character|GetStaticMesh)) "3.000000,3.000000,3.000000") false false)
    (Character|Jump)
    (Pawn|Input|AddMovementInput (- (Transformation|GetActorRightVector) "0,200.000000, 0") 1.0 false)
    (if (Math|Rotator|Equal(Rotator) (Transformation|GetWorldRotation (Variables|Character|GetStaticMesh)) "0,270.000000,90.000000" 0.0001)
      (Transformation|SetWorldLocationAndRotation (Variables|Character|GetStaticMesh) (+ (Transformation|GetWorldLocation (Variables|Character|GetStaticMesh)) "0.000000,300.000000, 0") "0,0.000000,90.000000" false false)
      (elif (Math|Rotator|Equal(Rotator) (Transformation|GetWorldRotation (Variables|Character|GetStaticMesh)) "0,180.000000,90.000000" 0.0001)
        (Transformation|SetWorldLocationAndRotation (Variables|Character|GetStaticMesh) (+ (Transformation|GetWorldLocation (Variables|Character|GetStaticMesh)) "300.000000,300.000000, 0") "0,0.000000,90.000000" false false)
        (elif (Math|Rotator|Equal(Rotator) (Transformation|GetWorldRotation (Variables|Character|GetStaticMesh)) "0,90.000000,90.000000" 0.0001)
          (Transformation|SetWorldLocationAndRotation (Variables|Character|GetStaticMesh) (+ (Transformation|GetWorldLocation (Variables|Character|GetStaticMesh)) "300.000000,0.000000, 0") "0,0.000000,90.000000" false false))))))

(event Input|ActionEvents|InputActionJumpRight
  (params (Key :type Key%20Structure :default "None"))
  (:Pressed
    (Transformation|SetWorldTransform (Variables|Character|GetStaticMesh) (Math|Transform|MakeTransform (Transformation|GetWorldLocation (Variables|Character|GetStaticMesh)) (Transformation|GetWorldRotation (Variables|Character|GetStaticMesh)) "3.000000,2.700000,3.000000") false false))
  (:Released
    (Transformation|SetWorldTransform (Variables|Character|GetStaticMesh) (Math|Transform|MakeTransform (Transformation|GetWorldLocation (Variables|Character|GetStaticMesh)) (Transformation|GetWorldRotation (Variables|Character|GetStaticMesh)) "3.000000,3.000000,3.000000") false false)
    (Character|Jump)
    (Pawn|Input|AddMovementInput (+ "0,200.000000, 0" (Transformation|GetActorRightVector)) 1.0 false)
    (if (Math|Rotator|Equal(Rotator) (Transformation|GetWorldRotation (Variables|Character|GetStaticMesh)) "0,270.000000,90.000000" 0.0001)
      (Transformation|SetWorldLocationAndRotation (Variables|Character|GetStaticMesh) (+ (Transformation|GetWorldLocation (Variables|Character|GetStaticMesh)) "-300.000000,0.000000, 0") "0,180.000000,90.000000" false false)
      (elif (Math|Rotator|Equal(Rotator) (Transformation|GetWorldRotation (Variables|Character|GetStaticMesh)) "0,90.000000,90.000000" 0.0001)
        (Transformation|SetWorldLocationAndRotation (Variables|Character|GetStaticMesh) (+ (Transformation|GetWorldLocation (Variables|Character|GetStaticMesh)) "0.000000,-300.000000, 0") "0,180.000000,90.000000" false false)
        (elif (Math|Rotator|Equal(Rotator) (Transformation|GetWorldRotation (Variables|Character|GetStaticMesh)) "0, 0,90.000000" 0.0001)
          (Transformation|SetWorldLocationAndRotation (Variables|Character|GetStaticMesh) (+ (Transformation|GetWorldLocation (Variables|Character|GetStaticMesh)) "-300.000000,-300.000000, 0") "0,180.000000,90.000000" false false))))))

(event Input|AxisEvents|InputAxisMoveForward
  (params (AxisValue :type Float%20%28single-precision%29))
  (Pawn|Input|AddMovementInput (Transformation|GetActorForwardVector) (* AxisValue (Variables|Default|GetMax%20Speed)) true))

(event Input|AxisEvents|InputAxisMoveRight
  (params (AxisValue :type Float%20%28single-precision%29))
  (Pawn|Input|AddMovementInput (Transformation|GetActorRightVector) (* AxisValue (Variables|Default|GetMax%20Speed)) true))

(fn ConstructionScript)

(fn Rotation
  (if (> (.x (Transformation|GetVelocity)) 0.0)
    (Transformation|SetActorRotation "0,-45.000000,0.000000")))

(fn CheckifChickenIsMovable)

(fn KeyPressedforMovement)